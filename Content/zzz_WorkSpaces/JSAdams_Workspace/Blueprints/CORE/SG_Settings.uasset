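; SG_Settings is a settings data object, apparently a SaveGame, that stores the player's Master, Music and SFX volume levels.
; GetAudioSettings returns all three values together, and a separate save function overwrites each one.
; The save functions only set variables, so writing to disk and applying the volumes to audio are not handled in these graphs.
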(fn `GetAudioSettings`
  (returns (MasterVolume :type "Float (double-precision)") (MusicVolume :type "Float (double-precision)") (`SFX Volume` :type "Float (double-precision)"))
  (return (`self.MasterVolume`) (`self.MusicVolume`) (`self.SFX Volume`)))

(fn `SaveMasterSound`
  (params (NewMasterSound :type "Float (double-precision)"))
  (set `self.MasterVolume` NewMasterSound)
  (return))

(fn `SaveMusicSound`
  (params (NewMusicSound :type "Float (double-precision)"))
  (set `self.MusicVolume` NewMusicSound)
  (return))

(fn `SaveSFXSound`
  (params (NewSFXVolume :type "Float (double-precision)"))
  (set `self.SFX Volume` NewSFXVolume)
  (return))