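; Level actor that runs the main menu flow and menu music, optionally starting both on BeginPlay with mouse cursor and Game-and-UI input.
; Open and close functions create and swap the Settings, Audio and Graphics widgets, re-adding the stored Settings widget when a submenu closes.
; Music plays on a stored 2D audio component that can fade out or take Master times Music volume from GI_UtahniGameInstance through a separate update function.
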(event `self.ReceiveBeginPlay`
  (bind _returnvalue (`GameplayStatics.GetPlayerController` 0))
  ;[0.02732 0.06848 0.04667] Add the Widget to View, Cast to the GI, Ask for Master Vol Mult it By Music Vol and spawn music at those levels, set the mouse ON and put us in input mode. (EchoDev)
  (if (`self.ShowMainMenuOnBeginPlay`)
    (bind _returnvalue_2 (`|CreateWidget` "/Game/zzz_WorkSpaces/JSAdams_Workspace/Widgets/WBP_MainMenu.WBP_MainMenu_C" (`GameplayStatics.GetPlayerController` 0)))
    (`UserWidget.AddToViewport` _returnvalue_2 0)
    (bind _output_get (set `self.MainMenuWidget` _returnvalue_2))
    (bind _returnvalue_3 (`GameplayStatics.SpawnSound2D` (`self.MenuMusic`) 1.0 1.0 0.0 null false false))
    (set `self.MenuMusicComp` _returnvalue_3)
    (bind _output_get_2 (set `PlayerController.bShowMouseCursor` true _returnvalue))
    (`WidgetBlueprintLibrary.SetInputMode_GameAndUIEx` _returnvalue _output_get "DoNotLock" _output_get_2)))

(fn `CloseAudioMenu`
  (bind _settingsmenuwidget (`self.SettingsMenuWidget`))
  (`Widget.RemoveFromParent` (`self.AudioMenuWidget`))
  (`/Engine/EditorBlueprintResources/StandardMacros.IsValid` _settingsmenuwidget
    (:`Is Valid`
      (`UserWidget.AddToViewport` _settingsmenuwidget 0))))

(fn `CloseGraphicsMenu`
  (bind _settingsmenuwidget (`self.SettingsMenuWidget`))
  (`Widget.RemoveFromParent` (`self.GraphicsMenuWidget`))
  (`/Engine/EditorBlueprintResources/StandardMacros.IsValid` _settingsmenuwidget
    (:`Is Valid`
      (`UserWidget.AddToViewport` _settingsmenuwidget 0))))

(fn `CloseSettingsMenu`
  (bind _settingsmenuwidget (`self.SettingsMenuWidget`))
  (bind _mainmenuwidget (`self.MainMenuWidget`))
  (`/Engine/EditorBlueprintResources/StandardMacros.IsValid` _settingsmenuwidget
    (:`Is Valid`
      (`Widget.RemoveFromParent` _settingsmenuwidget))
    (:`Is Not Valid`
      (`/Engine/EditorBlueprintResources/StandardMacros.IsValid` _mainmenuwidget
        (:`Is Valid`
          (`Widget.SetVisibility` _mainmenuwidget "Visible"))))))

(fn `FadeOutMenuMusic`
  (`AudioComponent.FadeOut` (`self.MenuMusicComp`) 1.5 0.0 "Linear"))

(fn `OpenAudioMenu`
  (bind _settingsmenuwidget (`self.SettingsMenuWidget`))
  (`/Engine/EditorBlueprintResources/StandardMacros.IsValid` _settingsmenuwidget
    (:`Is Valid`
      (`Widget.RemoveFromParent` _settingsmenuwidget))
    (:`Is Not Valid`
      _))
  (bind _returnvalue (`|CreateWidget` "/Game/zzz_WorkSpaces/JSAdams_Workspace/Widgets/WBP_AudioMenu.WBP_AudioMenu_C" (`GameplayStatics.GetPlayerController` 0)))
  (`UserWidget.AddToViewport` _returnvalue 50)
  (set `self.AudioMenuWidget` _returnvalue))

(fn `OpenGraphicsMenu`
  (bind _settingsmenuwidget (`self.SettingsMenuWidget`))
  (`/Engine/EditorBlueprintResources/StandardMacros.IsValid` _settingsmenuwidget
    (:`Is Valid`
      (`Widget.RemoveFromParent` _settingsmenuwidget))
    (:`Is Not Valid`
      _))
  (bind _returnvalue (`|CreateWidget` "/Game/zzz_WorkSpaces/JSAdams_Workspace/Widgets/WBP_GraphicsMenu.WBP_GraphicsMenu_C" (`GameplayStatics.GetPlayerController` 0)))
  (`UserWidget.AddToViewport` _returnvalue 50)
  (set `self.GraphicsMenuWidget` _returnvalue))

(fn `OpenSettingsMenu`
  (set `Widget.Visibility` "HitTestInvisible" (`self.MainMenuWidget`))
  (bind _returnvalue (`|CreateWidget` "/Game/zzz_WorkSpaces/JSAdams_Workspace/Widgets/WBP_SettingsMenu.WBP_SettingsMenu_C" (`GameplayStatics.GetPlayerController` 0)))
  (`UserWidget.AddToViewport` _returnvalue 0)
  (set `self.SettingsMenuWidget` _returnvalue))

(fn `UpdateMenuMusicVolume`
  (bind _asgi_utahni_game_instance (cast `/Game/zzz_WorkSpaces/JSAdams_Workspace/Blueprints/CORE/GI_UtahniGameInstance` (`GameplayStatics.GetGameInstance`)))
  (`AudioComponent.SetVolumeMultiplier` (`self.MenuMusicComp`) (* (`/Game/zzz_WorkSpaces/JSAdams_Workspace/Blueprints/CORE/GI_UtahniGameInstance.MasterVolume_0` _asgi_utahni_game_instance) (`/Game/zzz_WorkSpaces/JSAdams_Workspace/Blueprints/CORE/GI_UtahniGameInstance.MusicVolume_0` _asgi_utahni_game_instance))))

(fn `UserConstructionScript`)