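; BP_SplashFlowActor runs a splash screen, then opens the next level by name.
; On BeginPlay it enables input, adds the splash widget to the viewport and plays a 2D sound scaled by the game instance's master and SFX volumes.
; A timed delay or a skip press (Space, Enter, left mouse, gamepad bottom face button) calls AdvanceSplash, which uses a flag to prevent repeated level loads.
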(event `self.ReceiveBeginPlay`
  ;[0.02732 0.06848 0.04667] Get / Cast to GI Set Volume Levels ,Load WBP_ , Add to View, play sound, wait & Load next LVL
  (`self.EnableInput` (`GameplayStatics.GetPlayerController` 0))
  (bind _asgi_utahni_game_instance (cast `/Game/zzz_WorkSpaces/JSAdams_Workspace/Blueprints/CORE/GI_UtahniGameInstance` (`GameplayStatics.GetGameInstance`)))
  (bind _returnvalue (`|CreateWidget` (`self.SplashWidgetClass`)))
  (`UserWidget.AddToViewport` _returnvalue 0)
  (`GameplayStatics.SpawnSound2D` (`self.SplashSound`) (* (`/Game/zzz_WorkSpaces/JSAdams_Workspace/Blueprints/CORE/GI_UtahniGameInstance.MasterVolume_0` _asgi_utahni_game_instance) (`/Game/zzz_WorkSpaces/JSAdams_Workspace/Blueprints/CORE/GI_UtahniGameInstance.SFXVolume_0` _asgi_utahni_game_instance)) 1.0 0.0 null)
  (`KismetSystemLibrary.Delay` (`self.SplashDuration`))
  (`self.AdvanceSplash`))

(event `Key|SpaceBar`
  (params (Key :type "Key Structure"))
  (:`Pressed`
    (`self.AdvanceSplash` :!label _label)))

(event `Key|LeftMouseButton`
  (params (Key :type "Key Structure"))
  (:`Pressed`
    (goto _label)))

(event `Key|Enter`
  (params (Key :type "Key Structure"))
  (:`Pressed`
    (goto _label)))

(event `Key|Gamepad_FaceButton_Bottom`
  (params (Key :type "Key Structure"))
  (:`Pressed`
    (goto _label)))

(fn `AdvanceSplash`
  (if (not (`self.bAlreadyAdvancing`))
    (set `self.bAlreadyAdvancing` true)
    (`GameplayStatics.OpenLevel` (`self.NextLevelName`))))

(fn `UserConstructionScript`)